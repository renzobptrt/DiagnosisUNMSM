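; BP_paciente is a patient actor that takes on a random skeletal mesh and offers a placeholder E-key interaction.
; On BeginPlay it picks from SkmPosibles and sets ABP_02 or ABP_23 by mesh name, though the name check re-rolls the random index.
; Overlapping Caja_colision with ThirdPersonCharacter enables input and opens a Gate, which end overlap reverses.
; Releasing E only prints debug text, with a second print behind the Gate.
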(event `self.ReceiveBeginPlay`
  (bind _skm_posibles (`self.skm_posibles`))
  (bind _mesh (`self.Mesh`))
  (bind _output (`|GetArrayItem` _skm_posibles (`KismetMathLibrary.RandomInteger` (`KismetArrayLibrary.Array_Length` _skm_posibles))))
  (`SkinnedMeshComponent.SetSkinnedAssetAndUpdate` (`self.Mesh`) _output false)
  (if (== (`KismetSystemLibrary.GetDisplayName` _output) "ch02_nonpbr")
    (`SkeletalMeshComponent.SetAnimInstanceClass` _mesh "/Game/Paciente/ABP/ABP_02.ABP_02_C")
    (else
      (`SkeletalMeshComponent.SetAnimInstanceClass` _mesh "/Game/Paciente/ABP/ABP_23.ABP_23_C"))))

(event `Key|E`
  (params (Key :type "Key Structure"))
  (:`Released`
    (`KismetSystemLibrary.PrintString` "Hello")
    (`/Engine/EditorBlueprintResources/StandardMacros.Gate` true :!label _label
      (:`Exit`
        (`KismetSystemLibrary.PrintString` "Hello")))))

(event `self.caja_colision.OnComponentBeginOverlap`
  (params (OverlappedComponent :type "PrimitiveComponent Object Reference") (OtherActor :type "Actor Object Reference") (OtherComp :type "PrimitiveComponent Object Reference") (OtherBodyIndex :type Integer) (bFromSweep :type Boolean) (SweepResult :type "HitResult Structure (by ref)"))
  (cast `/Game/BluePrints/ThirdPersonCharacter` OtherActor)
  (`self.EnableInput` (`GameplayStatics.GetPlayerController` 0))
  (`KismetSystemLibrary.PrintString` "overlap")
  (goto _label :!via `Open`))

(event `self.caja_colision.OnComponentEndOverlap`
  (params (OverlappedComponent :type "PrimitiveComponent Object Reference") (OtherActor :type "Actor Object Reference") (OtherComp :type "PrimitiveComponent Object Reference") (OtherBodyIndex :type Integer))
  (`self.DisableInput` (`GameplayStatics.GetPlayerController` 0))
  (`KismetSystemLibrary.PrintString` "no overlap")
  (goto _label :!via `Close`))

(fn `UserConstructionScript`)