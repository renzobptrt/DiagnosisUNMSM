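; Patient actor for a medical diagnosis game, with a random female name and illness that determine its temperature, lung scan and stomach ultrasound results.
; While FollowPlayer is set, it re-issues AI moves toward the player on a short delayed loop, holding position when close.
; Flag-gated reveal events append results to an on-screen text via MostrarNuevoDato; the temperature check is inverted, requiring MostroTemp to already be true.
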(event `self.ReceiveBeginPlay`
  (`self.Asignar_Datos`))

(event `follow player`
  (bind _jugador_ref (`self.Jugador_ref`))
  ;[1 1 1] follow player
  (if (`self.followPlayer?`)
    (if (>= (`self.GetDistanceTo` _jugador_ref) 400.0)
      (`|AIMoveTo` self (0.0 0.0 0.0) _jugador_ref
        (:`then`
          _))
      (else
        (`|AIMoveTo` self (0.0 0.0 0.0) self
          (:`then`
            _))))
    (`KismetSystemLibrary.Delay` 0.2)
    (`self.follow player`)))

(event `mostrar_temperatura`
  ;[1 1 1] mostrar datos
  (if (`self.mostro_temp`)
    (`self.Mostrar Nuevo Dato` (`KismetStringLibrary.Conv_IntToString` (`self.temperatura`)))
    (set `self.mostro_temp` true)))

(event `mostrar_pulmon_estado`
  ;[1 1 1] mostrar datos
  (if (not (`self.mostro_pulmon`))
    (if (`self.scaner pulmo limpio?`)
      (`self.Mostrar Nuevo Dato` "pulmón limpio")
      (else
        (`self.Mostrar Nuevo Dato` "pulmón infectado")))
    (set `self.mostro_pulmon` true)))

(event `mostrar_estado_estomago`
  ;[1 1 1] mostrar datos
  (if (not (`self.mostro_eco`))
    (if (`self.ecografia limpia?`)
      (`self.Mostrar Nuevo Dato` "estomago limpio")
      (else
        (`self.Mostrar Nuevo Dato` "estomago infectado")))
    (set `self.mostro_eco` true)))

(fn `Asignar_Datos`
  (bind _asthird_person_character (cast `/Game/BluePrints/ThirdPersonCharacter` (`GameplayStatics.GetPlayerCharacter` 0)))
  (set `self.Jugador_ref` _asthird_person_character)
  (`self.follow player`)
  (bind _output_get (set `self.nombre` (`|GetArrayItem` (`self.nombres femeninos`) (`KismetMathLibrary.RandomInteger` 2))))
  (`self.Mostrar Nuevo Dato` _output_get)
  (set `self.enfermedad` (`|GetArrayItem` (`self.enfermedades`) (`KismetMathLibrary.RandomInteger` 2)))
  (if (`KismetStringLibrary.NotEqual_StrStr` (`self.enfermedad`) "gastritis")
    (set `self.temperatura` 38)
    (else
      (set `self.temperatura` 36)))
  (if (`KismetStringLibrary.EqualEqual_StrStr` (`self.enfermedad`) "gastritis")
    (set `self.ecografia limpia?` false)
    (else
      (set `self.ecografia limpia?` true)))
  (if (`KismetStringLibrary.EqualEqual_StrStr` (`self.enfermedad`) "gripe")
    (set `self.scaner pulmo limpio?` false)
    (else
      (set `self.scaner pulmo limpio?` true)))
  (set `self.es hombre?` false))

(fn `Mostrar Nuevo Dato`
  (params (Texto :type String))
  (locals (NewLocalVar_3 :type String))
  (bind _texto_visible (`self.texto_visible`))
  (bind _output_get (set `self.NewVar_0` ""))
  (if (`KismetTextLibrary.EqualEqual_TextText` _output_get _texto_visible)
    (bind _output_get_2 (set `self.texto_visible` (`KismetTextLibrary.Conv_StringToText` Texto)))
    (else
      (set `self.texto_visible` (`KismetTextLibrary.Conv_StringToText` (`KismetStringLibrary.Concat_StrStr` (`KismetStringLibrary.Concat_StrStr` (`KismetTextLibrary.Conv_TextToString` _texto_visible) " \n") Texto)))))
  (`TextRenderComponent.K2_SetText` (`self.texto_datos`) _output_get_2))

(fn `UserConstructionScript`
  (locals (NewLocalVar_0 :type "Object Object Reference") (NewLocalVar_1 :type "Object Object Reference") (NewLocalVar_2 :type "Object Object Reference")))