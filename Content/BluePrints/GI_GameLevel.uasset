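; GI_GameLevel, a game instance by its prefix, tracks level progress and patient results for the game.
; It keeps separate counters for correct (PacientesAcertados) and failed (PacientesFallidos) patients, each raised by one through its own function.
; Other functions advance CurrentLevel, reset it to zero, or set MaxLevels from a passed value.
; No function here resets the patient counters or checks the level against the maximum.
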(fn `AddNewLevel`
  (set `self.CurrentLevel` (+ (`self.CurrentLevel`) 1)))

(fn `AddPacienteAcertado`
  (set `self.PacientesAcertados` (+ (`self.PacientesAcertados`) 1)))

(fn `AddPacienteFallido`
  (set `self.PacientesFallidos` (+ (`self.PacientesFallidos`) 1)))

(fn `ResetLevel`
  (set `self.CurrentLevel` 0))

(fn `SetMaxLevels`
  (params (CurrentMaxLevels :type Integer))
  (set `self.MaxLevels` CurrentMaxLevels))