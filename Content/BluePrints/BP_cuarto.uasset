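; BP_cuarto is a room that takes in a BP_paciente and sends it to the room's center.
; BoxColision counts overlaps of any actor; once Cantidad reaches two, the next patient overlap resets it and calls PacienteEntro.
; That patient's capsule ignores Pawn collision, AIMoveTo sends it to Centro, and FollowPlayer is cleared without waiting for arrival.
; Leaving the box restores Pawn blocking on any patient.
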(event `self.box colision.OnComponentBeginOverlap`
  (params (OverlappedComponent :type "PrimitiveComponent Object Reference") (OtherActor :type "Actor Object Reference") (OtherComp :type "PrimitiveComponent Object Reference") (OtherBodyIndex :type Integer) (bFromSweep :type Boolean) (SweepResult :type "HitResult Structure (by ref)"))
  (if (>= (`self.cantidad`) 2)
    (bind _asbp_paciente (cast `/Game/BluePrints/BP_paciente` OtherActor))
    (set `self.cantidad` 0)
    (bind _output_get (set `self.paciente ref` _asbp_paciente))
    (`KismetSystemLibrary.PrintString` "llamando")
    (`self.PacienteEntro` _output_get)
    (`PrimitiveComponent.SetCollisionResponseToChannel` (`Character.CapsuleComponent` (`self.paciente ref`)) "ECC_Pawn" "ECR_Ignore")
    (`|AIMoveTo` (`self.paciente ref`) (`SceneComponent.K2_GetComponentLocation` (`self.centro`)) null
      (:`then`
        (set `/Game/BluePrints/BP_paciente.followPlayer?` false (`self.paciente ref`))))
    (else
      (`/Engine/EditorBlueprintResources/StandardMacros.IncrementInt` (`self.cantidad`)))))

(event `self.box colision.OnComponentEndOverlap`
  (params (OverlappedComponent :type "PrimitiveComponent Object Reference") (OtherActor :type "Actor Object Reference") (OtherComp :type "PrimitiveComponent Object Reference") (OtherBodyIndex :type Integer))
  (bind _asbp_paciente (cast `/Game/BluePrints/BP_paciente` OtherActor))
  (`PrimitiveComponent.SetCollisionResponseToChannel` (`Character.CapsuleComponent` _asbp_paciente) "ECC_Pawn" "ECR_Block"))

(fn `PacienteEntro`
  (params (Paciente :type "/Game/BluePrints/BP_paciente Object Reference")))

(fn `UserConstructionScript`)