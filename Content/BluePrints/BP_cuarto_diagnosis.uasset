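; Diagnosis room Blueprint that opens a diagnosis selection screen when a patient enters.
; PacienteEntro prints a debug message, calls MostrarSeleccion, then passes the patient to the returned widget.
; MostrarSeleccion creates and stores a WB_Diagnosis widget, adds it to the player screen, shows the cursor and switches input to UI-only.
; Its event graph is inactive, so PacienteEntro has no caller within this Blueprint.
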(fn `MostrarSeleccion`
  (returns (HUD :type "/Game/BluePrints/HUD/WB_Diagnosis Object Reference"))
  (bind _returnvalue (`GameplayStatics.GetPlayerController` 0))
  (bind _hud_seleccion (`self.HUD seleccion`))
  (bind _returnvalue_2 (`|CreateWidget` "/Game/BluePrints/HUD/WB_Diagnosis.WB_Diagnosis_C" _returnvalue))
  (bind _output_get (set `self.HUD seleccion` _returnvalue_2))
  (`UserWidget.AddToPlayerScreen` _output_get 0)
  (set `PlayerController.bShowMouseCursor` true _returnvalue)
  (`WidgetBlueprintLibrary.SetInputMode_UIOnlyEx` _returnvalue _hud_seleccion)
  (return _hud_seleccion))

(fn `PacienteEntro`
  (params (Paciente :type "/Game/BluePrints/BP_paciente Object Reference"))
  (`KismetSystemLibrary.PrintString` "paciente entro")
  (bind _hud (`self.MostrarSeleccion`))
  (set `/Game/BluePrints/HUD/WB_Diagnosis.Paciente` Paciente _hud))

(fn `UserConstructionScript`
  (`parent.UserConstructionScript`))