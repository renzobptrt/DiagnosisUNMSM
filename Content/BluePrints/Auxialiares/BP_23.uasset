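; BP_23 is an auxiliary Blueprint that sets itself up as a male individual with a randomly chosen name.
; On BeginPlay it runs the parent logic, sets EsHombre to true and picks Nombre at random from the first two entries of NombresMasculinos.
; The name is converted to text and shown through TextoDatos.
; The construction script only calls its parent, and overlap and tick events are unused.
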(event `self.ReceiveBeginPlay`
  (`parent.ReceiveBeginPlay`)
  (set `self.es hombre?` true)
  (bind _output_get (set `self.nombre` (`|GetArrayItem` (`self.nombres masculinos`) (`KismetMathLibrary.RandomInteger` 2))))
  (bind _output_get_2 (set `self.texto a mostrar` (`KismetTextLibrary.Conv_StringToText` _output_get)))
  (`TextRenderComponent.K2_SetText` (`self.texto_datos`) _output_get_2))

(fn `UserConstructionScript`
  (`parent.UserConstructionScript`))