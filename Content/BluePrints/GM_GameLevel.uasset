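; GM_GameLevel is the game mode that runs timed levels in which the player must reach a patient goal before moving on.
; Construction sends the DataLevels row count to GI_GameLevel; BeginPlay loads the current level's time and goal, shows an intro widget, then starts the HUD and countdown.
; At timeout, meeting the goal reopens GameLevel as the next level, while failing or passing the last level shows the game-over screen.
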(event `self.ReceiveBeginPlay`
  (`self.SetLevel`)
  (bind _returnvalue (`|CreateWidget` "/Game/BluePrints/HUD/WB_CurrentLevel.WB_CurrentLevel_C"))
  (bind _output_get (set `self.WidgetLevel Reference` _returnvalue))
  (`UserWidget.AddToViewport` _output_get 0)
  (`KismetSystemLibrary.Delay` 3.0)
  (`Widget.RemoveFromParent` (`self.WidgetLevel Reference`))
  (`self.StartLevel`))

(event `StartLevel`
  (bind _returnvalue (`|CreateWidget` "/Game/BluePrints/HUD/WB_GameLevel.WB_GameLevel_C"))
  (bind _output_get (set `self.WidgetReference` _returnvalue))
  (`UserWidget.AddToViewport` _output_get 0)
  (`KismetSystemLibrary.K2_SetTimerDelegate` (delegate `CountDown`) 1.0 true))

(event `CountDown`
  (bind _result (`/Engine/EditorBlueprintResources/StandardMacros.DecrementInt` (`self.TimeRemaining`))
    (:`  `
      (if (< _result 0)
        (if (<= (`self.GoalPaccient`) (`/Game/BluePrints/GI_GameLevel.PacientesAcertados` (`self.GameInstance Ref`)))
          (`self.GoToNewLevel`)
          (else
            (`self.GoToGameOver`)))))))

(event `GoToNewLevel`
  (`/Game/BluePrints/GI_GameLevel.AddNewLevel` (`self.GameInstance Ref`))
  (if (<= (`/Game/BluePrints/GI_GameLevel.CurrentLevel` (`self.GameInstance Ref`)) (`/Game/BluePrints/GI_GameLevel.MaxLevels` (`self.GameInstance Ref`)))
    (`GameplayStatics.OpenLevel` "GameLevel")
    (else
      (`self.GoToGameOver`))))

(event `GoToGameOver`
  (bind _returnvalue (`GameplayStatics.GetPlayerController` 0))
  (`Widget.RemoveFromParent` (`self.WidgetReference`))
  (set `PlayerController.bShowMouseCursor` true _returnvalue)
  (`WidgetBlueprintLibrary.SetInputMode_UIOnlyEx` _returnvalue null)
  (bind _returnvalue_2 (`|CreateWidget` "/Game/BluePrints/HUD/WB_GameOver.WB_GameOver_C"))
  (`UserWidget.AddToViewport` _returnvalue_2 0))

(fn `SetLevel`
  (bind _outrownames (`DataTableFunctionLibrary.GetDataTableRowNames` (`self.DataLevels`)))
  (bind _returnvalue (`|GetDataTableRow` (`self.DataLevels`) (`|GetArrayItem` _outrownames (- (`/Game/BluePrints/GI_GameLevel.CurrentLevel` (`self.GameInstance Ref`)) 1)))
    (:`then`
      (bind (_numlevel _timeremaining _goalpaccient) (break `/Game/Data/S_Level` _returnvalue))
      (set `self.TimeRemaining` _timeremaining)
      (set `self.GoalPaccient` _goalpaccient))))

(fn `UserConstructionScript`
  (locals (CurrentMaxLevels :type Integer :default 0))
  (bind _outrownames (`DataTableFunctionLibrary.GetDataTableRowNames` (`self.DataLevels`)))
  (set `local.CurrentMaxLevels` (`KismetArrayLibrary.Array_Length` _outrownames))
  (bind _asgi_game_level (cast `/Game/BluePrints/GI_GameLevel` (`GameplayStatics.GetGameInstance`)))
  (bind _output_get (set `self.GameInstance Ref` _asgi_game_level))
  (`/Game/BluePrints/GI_GameLevel.SetMaxLevels` _output_get (`local.CurrentMaxLevels`)))